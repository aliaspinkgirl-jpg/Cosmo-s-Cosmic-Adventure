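; Game instance for Archie Adventure that holds a reference to the current music and exposes a PlayMusic event.
; With no valid Music, the event spawns a 2D sound from the given audio, volume and level-transition persistence, stores it and plays it.
; With valid Music, it only clears the reference, neither stopping that sound nor starting the new one.
; An IsPlaying check is left unconnected and never runs.
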(event `Play Music`
  (params (Audio :type "SoundBase Object Reference") (Volume :type "Float (single-precision)") (bPersistAcrossLevelTransition :type Boolean))
  (`/Engine/EditorBlueprintResources/StandardMacros.IsValid` (`self.Music`)
    (:`Is Valid`
      (if true
        (bind _output_get (set `self.Music` null))))
    (:`Is Not Valid`
      (bind _returnvalue (`GameplayStatics.SpawnSound2D` Audio Volume 1.0 0.0 null bPersistAcrossLevelTransition))
      (bind _output_get_2 (set `self.Music` _returnvalue))
      (`AudioComponent.Play` _output_get_2 0.0))))