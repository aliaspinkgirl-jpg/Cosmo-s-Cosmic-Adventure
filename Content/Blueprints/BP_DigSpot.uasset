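; BP_DigSpot is a diggable spot actor that the player uncovers with a dig ability.
; When BP_Player overlaps the Digtrigger while its dig ability is active and the spot is not yet dug, the player plays its dig animation.
; After a two-second delay, the Dirt component is destroyed and the spot is marked as dug.
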(event `self.Digtrigger.OnComponentBeginOverlap`
  (params (OverlappedComponent :type "PrimitiveComponent Object Reference") (OtherActor :type "Actor Object Reference") (OtherComp :type "PrimitiveComponent Object Reference") (OtherBodyIndex :type Integer) (bFromSweep :type Boolean) (SweepResult :type "HitResult Structure (by ref)"))
  (bind _asbp_player (cast `/Game/Blueprints/BP_Player` OtherActor))
  (if (and (`/Game/Blueprints/BP_Player.bDigAbilityActive` _asbp_player) (not (`self.bIsDug`)))
    (`/Game/Blueprints/BP_Player.DigAnimation` _asbp_player)
    (`KismetSystemLibrary.Delay` 2.0)
    (`/Engine/EditorBlueprintResources/StandardMacros.IsValid` "/Game/Sunnyland/environment/props/Dirt.Dirt"
      (:`Is Valid`
        (`ActorComponent.K2_DestroyComponent` (`self.Dirt`))
        (set `self.bIsDug` true)))))

(fn `UserConstructionScript`)